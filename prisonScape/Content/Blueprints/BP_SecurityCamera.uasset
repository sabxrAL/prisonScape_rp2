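; Security camera that sweeps back and forth and ends the game when its detection box is overlapped.
; A timeline ping-pongs the camera's yaw, while a per-tick visibility trace from the scene capture places a decal where its view lands.
; Any overlap switches the decal to a caught material, stops the sweep, plays a sound, freezes time and shows the game-over UI.
; AI blackboard alert nodes exist but never run.
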(event `self.ReceiveBeginPlay`
  (bind (_relativerotation_roll _relativerotation_pitch) (`KismetMathLibrary.BreakRotator` (`SceneComponent.RelativeRotation` (`self.camera`))))
  (bind _asbp_game_instance (cast `/Game/Blueprints/BP_GameInstance` (`GameplayStatics.GetGameInstance`)))
  (set `self.GameInstanceRef` _asbp_game_instance)
  (bind (_direction _moving_value) (`Timeline|Timeline` :!label _label)
    (:`Update`
      (`SceneComponent.K2_SetRelativeRotation` (`self.camera`) (`KismetMathLibrary.RLerp` (`KismetMathLibrary.MakeRotator` _relativerotation_roll _relativerotation_pitch -45.0) (`KismetMathLibrary.MakeRotator` _relativerotation_roll _relativerotation_pitch 45.0) _moving_value) false false))
    (:`Finished`
      (if (`self.ItRestart?`)
        (set `self.ItRestart?` false)
        (goto _label)
        (else
          (set `self.ItRestart?` true)
          (goto _label :!via `Reverse`))))))

(event `Block Timeline`
  (goto _label :!via `Stop`))

(event `self.ReceiveTick`
  (params (DeltaSeconds :type "Float (single-precision)"))
  (bind _returnvalue (`SceneComponent.K2_GetComponentLocation` (`self.SceneCaptureComponent2D`)))
  (bind _outhit (`KismetSystemLibrary.LineTraceSingle` :`Start` _returnvalue :`End` (+ (* (`SceneComponent.GetForwardVector` (`self.SceneCaptureComponent2D`)) 800.0) _returnvalue) :`TraceChannel` "TraceTypeQuery1" :`DrawDebugType` "ForOneFrame"))
  (bind (_bblockinghit _binitialoverlap _time _distance _location _impactpoint _normal _impactnormal) (`GameplayStatics.BreakHitResult` _outhit))
  (`SceneComponent.K2_SetWorldLocationAndRotation` (`self.Decal`) _impactpoint (`KismetMathLibrary.Conv_VectorToRotator` _impactnormal) false false))

(event `self.Box.OnComponentBeginOverlap`
  (params (OverlappedComponent :type "PrimitiveComponent Object Reference") (OtherActor :type "Actor Object Reference") (OtherComp :type "PrimitiveComponent Object Reference") (OtherBodyIndex :type Integer) (bFromSweep :type Boolean) (SweepResult :type "HitResult Structure (by ref)"))
  (`DecalComponent.SetDecalMaterial` (`self.Decal`) "/Game/Materials/DecalMaterials/Decal_Caught.Decal_Caught")
  (`self.Block Timeline`)
  (`GameplayStatics.PlaySound2D` "/Game/Audio/kauasilbershlachparodes-shutter-click-3-494029.kauasilbershlachparodes-shutter-click-3-494029" 1.0 1.0 0.0 null null)
  (`GameplayStatics.SetGlobalTimeDilation` 0.0)
  (bind _returnvalue (`|CreateWidget` "/Game/UI/WB_GameOver.WB_GameOver_C"))
  (`UserWidget.AddToViewport` _returnvalue 0)
  (bind _returnvalue_2 (`InputDeviceLibrary.GetPlayerControllerFromInputDevice` (struct)))
  (set `PlayerController.bShowMouseCursor` true _returnvalue_2)
  (`WidgetBlueprintLibrary.SetInputMode_UIOnlyEx` _returnvalue_2 null))

(fn `UserConstructionScript`)