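; BP_AccessDoor is a door that opens only for a player holding its required card.
; Box overlaps cross-link the door and BP_CHARACTER through PlayerInRange and DoorInRange; end overlap sets the same references instead of clearing them.
; TryOpenDoor checks the player's card, then destroys the door as a placeholder for an opening animation, or prints a wrong-card message.
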(event `self.Box.OnComponentBeginOverlap`
  (params (OverlappedComponent :type "PrimitiveComponent Object Reference") (OtherActor :type "Actor Object Reference") (OtherComp :type "PrimitiveComponent Object Reference") (OtherBodyIndex :type Integer) (bFromSweep :type Boolean) (SweepResult :type "HitResult Structure (by ref)"))
  (bind _asbp_character (cast `/Game/ThirdPerson/Blueprints/BP_CHARACTER` OtherActor))
  (set `self.PlayerInRange` _asbp_character)
  (set `/Game/ThirdPerson/Blueprints/BP_CHARACTER.DoorInRange` self _asbp_character)
  (`KismetSystemLibrary.PrintString` "doorinrange"))

(event `self.Box.OnComponentEndOverlap`
  (params (OverlappedComponent :type "PrimitiveComponent Object Reference") (OtherActor :type "Actor Object Reference") (OtherComp :type "PrimitiveComponent Object Reference") (OtherBodyIndex :type Integer))
  (bind _asbp_character (cast `/Game/ThirdPerson/Blueprints/BP_CHARACTER` OtherActor))
  (set `self.PlayerInRange` _asbp_character)
  (set `/Game/ThirdPerson/Blueprints/BP_CHARACTER.DoorInRange` self _asbp_character))

(fn `TryOpenDoor`
  (`/Engine/EditorBlueprintResources/StandardMacros.IsValid` (`self.PlayerInRange`)
    (:`Is Valid`
      (bind _returnvalue (`/Game/ThirdPerson/Blueprints/BP_CHARACTER.HasCard` (`self.PlayerInRange`) (`self.RequiredCard`)))
      (if _returnvalue
        (if (not (`self.bIsOpen`))
          (set `self.bIsOpen` true)
          ; Esto hay que cambiarlo cuando se tenga animcacion de la puerta abriendose
          (`self.K2_DestroyActor`))
        (else
          (`KismetSystemLibrary.PrintString` "No tienes la tarjeta correcta"))))))

(fn `UserConstructionScript`)