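; Bp_Bricks is an interactable bricks actor that the player hides or destroys by pressing E when nearby.
; A trigger overlap with BP_CHARACTER sets a proximity flag, enables player 0's input on the actor and shows prompt text, reversing all three on exit.
; E hides the mesh if flagged visible; otherwise it makes the mesh visible and immediately destroys the actor.
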(event `self.Trigger_ifClose.OnComponentBeginOverlap`
  (params (OverlappedComponent :type "PrimitiveComponent Object Reference") (OtherActor :type "Actor Object Reference") (OtherComp :type "PrimitiveComponent Object Reference") (OtherBodyIndex :type Integer) (bFromSweep :type Boolean) (SweepResult :type "HitResult Structure (by ref)"))
  ; Detect if close
  (cast `/Game/ThirdPerson/Blueprints/BP_CHARACTER` OtherActor)
  (if true
    (set `self.BJugadorCerca` true)
    (`self.EnableInput` (`GameplayStatics.GetPlayerController` 0))
    (`SceneComponent.SetHiddenInGame` (`self.Bricks_Text`) false false)))

(event `self.ReceiveBeginPlay`)

(event `self.Trigger_ifClose.OnComponentEndOverlap`
  (params (OverlappedComponent :type "PrimitiveComponent Object Reference") (OtherActor :type "Actor Object Reference") (OtherComp :type "PrimitiveComponent Object Reference") (OtherBodyIndex :type Integer))
  ; Detect if close
  (cast `/Game/ThirdPerson/Blueprints/BP_CHARACTER` OtherActor)
  (if true
    (set `self.BJugadorCerca` false)
    (`self.DisableInput` (`GameplayStatics.GetPlayerController` 0))
    (`SceneComponent.SetHiddenInGame` (`self.Bricks_Text`) true false)))

(event `Key|E`
  (params (Key :type "Key Structure"))
  ;[0.02604 0.02604 0.02604] Press e
  (:`Pressed`
    (if (`self.BJugadorCerca`)
      (if (`self.BVisible`)
        (`SceneComponent.SetVisibility` (`self.StaticMesh`) false false)
        (set `self.BVisible` false)
        (else
          (`SceneComponent.SetVisibility` (`self.StaticMesh`) true false)
          (set `self.BVisible` true)
          (`self.K2_DestroyActor`))))))

(fn `UserConstructionScript`)