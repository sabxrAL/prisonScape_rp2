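; BP_SandwichPart is a collectible sandwich ingredient that the player picks up by walking into it.
; When its Box overlaps BP_CHARACTER, it passes its SandwichPartType to the character and destroys itself.
; If the character then has every part, it unhides all BP_SandwichFinal actors in the level, revealing the finished sandwich.
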(event `self.Box.OnComponentBeginOverlap`
  (params (OverlappedComponent :type "PrimitiveComponent Object Reference") (OtherActor :type "Actor Object Reference") (OtherComp :type "PrimitiveComponent Object Reference") (OtherBodyIndex :type Integer) (bFromSweep :type Boolean) (SweepResult :type "HitResult Structure (by ref)"))
  (bind _asbp_character (cast `/Game/ThirdPerson/Blueprints/BP_CHARACTER` OtherActor))
  (`/Game/ThirdPerson/Blueprints/BP_CHARACTER.AddSandwichPart` _asbp_character (`self.SandwichPartType`))
  (`self.K2_DestroyActor`)
  (bind _retrunvalue (`/Game/ThirdPerson/Blueprints/BP_CHARACTER.HasAllSandwichParts` _asbp_character))
  (if _retrunvalue
    (bind _outactors (`GameplayStatics.GetAllActorsOfClass` "/Game/Blueprints/BP_SandwichFinal.BP_SandwichFinal_C"))
    (for _array_element _outactors
      (`self.SetActorHiddenInGame` _array_element false))))

(fn `UserConstructionScript`)