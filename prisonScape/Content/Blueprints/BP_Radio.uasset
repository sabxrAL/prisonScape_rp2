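; BP_Radio is an interactable radio that toggles on and off and can draw AI attention through noise.
; Interact checks IsRadioOn and either stops Station1 or plays a sound at the mesh, waits briefly, then starts Station1 from the beginning.
; Switching on also reports a single "Radio"-tagged noise event at the mesh location, with the radio as instigator and a limited range.
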(event `/Game/Blueprints/BPI_Interface.Interact`
  (params (NewParam :type "/Game/Blueprints/BP_Locker Object Reference"))
  ; TURN RADIO ON
  (if (`self.IsRadioOn?`)
    (`AudioComponent.Stop` (`self.Station_1`))
    (set `self.IsRadioOn?` false)
    (else
      (`GameplayStatics.PlaySoundAtLocation` null (`SceneComponent.K2_GetComponentLocation` (`self.StaticMesh`)) (struct) 1.0 1.0 0.0 null null null null)
      (`KismetSystemLibrary.Delay` 0.5)
      (`AudioComponent.Play` (`self.Station_1`) 0.0)
      (set `self.IsRadioOn?` true)
      (`AISense_Hearing.ReportNoiseEvent` (`SceneComponent.K2_GetComponentLocation` (`self.StaticMesh`)) 1.0 self 3000.0 "Radio"))))

(fn `UserConstructionScript`)