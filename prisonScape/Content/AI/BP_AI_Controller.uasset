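; AI controller that runs the BT_AI behavior tree and sends the AI to investigate when it perceives a stimulus.
; On a successful perception update, it sets the HasHeardNoise blackboard key and puts BP_Radio in InvestigateActor, whatever the stimulus source or sense.
; Neither key is cleared here, and debug strings print along the way.
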(event `self.ReceiveBeginPlay`
  (`self.RunBehaviorTree` "/Game/AI/BT_AI.BT_AI"))

(event `self.AIPerception.OnTargetPerceptionUpdated`
  (params (Actor :type "Actor Object Reference") (Stimulus :type "AIStimulus Structure"))
  (if (`.bSuccessfullySensed` (break `AIStimulus` Stimulus))
    (`KismetSystemLibrary.PrintString` "percepted")
    (`BlackboardComponent.SetValueAsBool` (`AIBlueprintHelperLibrary.GetBlackboard` (`AIBlueprintHelperLibrary.GetAIController` self)) "HasHeardNoise" true)
    (`KismetSystemLibrary.PrintString` "rlivhriu")
    (`BlackboardComponent.SetValueAsObject` (`AIBlueprintHelperLibrary.GetBlackboard` (`AIBlueprintHelperLibrary.GetAIController` self)) "InvestigateActor" "/Game/Blueprints/BP_Radio.BP_Radio")
    (`KismetSystemLibrary.PrintString` "works")))

(fn `UserConstructionScript`)